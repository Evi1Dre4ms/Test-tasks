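; BP_Turtle is an AI-moved turtle character that travels to a target location, then plays a finish sound and effect before destroying itself.
; Move selects a mode: direct, stop-and-go, or stop-and-backtrack toward the start.
; The stepped modes interrupt AIMoveTo with timed StopActiveMovement calls and use its Fail output to loop.
; BeginPlay triggers spawn sound and particles, while Tick toggles footstep audio by velocity.
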(event Custom|Move
  (params (Movement%20Mode :type BP_MovementMode%20Enum :default "NewEnumerator0") (TargetLocation :type Vector))
  (Utilities|FlowControl|Delay 0.4)
  (Variables|Default|SetDestinationLocation TargetLocation)
  (Variables|Default|SetInitialLocation (Transformation|GetActorLocation))
  (switch Utilities|FlowControl|Switch|SwitchonBP_MovementMode Movement%20Mode
    (:NewEnumerator0
      (AI|AIMoveTo self (Variables|Default|GetDestinationLocation) 0 2.0 false
        (:OnSuccess
          (Utilities|DestroyonFinish))))
    (:NewEnumerator1
      (AI|AIMoveTo self (Variables|Default|GetDestinationLocation) 0 5.0 false :!label _label
        (:then
          (Utilities|FlowControl|Delay 1.0)
          (Class|NavMovementComponent|StopActiveMovement (Variables|Character|GetCharacterMovement)))
        (:OnSuccess
          (Utilities|DestroyonFinish))
        (:OnFail
          (Utilities|FlowControl|Delay 0.5)
          (goto _label))))
    (:NewEnumerator2
      (AI|AIMoveTo self (Variables|Default|GetDestinationLocation) 0 5.0 false :!label _label_2
        (:then
          (Utilities|FlowControl|Delay 1.0)
          (Class|NavMovementComponent|StopActiveMovement (Variables|Character|GetCharacterMovement)))
        (:OnSuccess
          (Utilities|DestroyonFinish))
        (:OnFail
          (AI|AIMoveTo self (Variables|Default|GetInitialLocation) 0 5.0 false
            (:then
              (Utilities|FlowControl|Delay 0.5)
              (Class|NavMovementComponent|StopActiveMovement (Variables|Character|GetCharacterMovement)))
            (:OnFail
              (goto _label_2))))))))

(event EventBeginPlay
  (Audio|PlaySound2D "/Game/Sounds/retro-game-notification.retro-game-notification" 1.0 1.0 0.0 0 0)
  (Components|Activation|Activate (Variables|Default|GetSpawnEffect) false)
  (Components|Activation|Activate (Variables|Default|GetWalkingEffect) false))

(event Collision|EventActorBeginOverlap
  (params (OtherActor :type Actor%20Object%20Reference)))

(event EventTick
  (params (DeltaSeconds :type Float%20%28single-precision%29))
  (bind _footsteps (Variables|Default|GetFootsteps))
  (if (> (Math|Vector|VectorLength (Transformation|GetVelocity self)) 0.0)
    (Audio|Components|Audio|Play _footsteps 0.0)
    (else
      (Audio|Components|Audio|Stop _footsteps))))

(fn ConstructionScript)